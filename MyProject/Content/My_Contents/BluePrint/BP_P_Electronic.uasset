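; BP_P_Electronic is an AI-controlled electron that runs the MyBT behavior tree on BeginPlay through its AIController.
; The construction script snaps its Sphere to the Arrow, sets it to overlap all channels and stores a dynamic instance of the electron material.
; GetDestination is a stub returning the zero vector, while GetOverlapActor returns overlapping actors.
; A loop meant to filter those by the "Shinnkai" tag is disconnected and never runs.
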(event `self.ReceiveBeginPlay`
  (bind _asaicontroller (cast `AIController` (`self.GetController`)))
  (`AIController.RunBehaviorTree` _asaicontroller (`self.My_BT`)))

(fn `Get_Destination`
  (returns (Destination :type "Vector Structure"))
  (return (0.0 0.0 0.0)))

(fn `Get_Overlap_Actor`
  (params (My :type "Actor Object Reference"))
  (returns (Overlap_Actor :type "Array of Actor Object Reference"))
  (locals (overlap_actors_has_tag :type "Array of Actor Object Reference"))
  (bind _asbp_p_electronic (cast `/Game/My_Contents/BluePrint/BP_P_Electronic` My))
  (return (`self.GetOverlappingActors` _asbp_p_electronic null)))

(fn `UserConstructionScript`
  (locals (NewLocalVar_0 :type "SphereComponent Object Reference"))
  (bind _sphere (`self.Sphere`))
  (`|ExecutionSequence`
    (:`then_0`
      ;[1 1 1] 電子の各種設定
      (`SceneComponent.K2_AttachToComponent` (`self.Sphere`) (`self.Arrow`) "None" "SnapToTarget" "SnapToTarget" "SnapToTarget" true)
      (`PrimitiveComponent.SetMaterial` _sphere 0 "/Game/My_Contents/Materials/MT_Opaque_Inst.MT_Opaque_Inst")
      (`PrimitiveComponent.SetCollisionResponseToAllChannels` _sphere "ECR_Overlap")
      (bind _returnvalue (`PrimitiveComponent.CreateDynamicMaterialInstance` _sphere 0 "/Game/My_Contents/Materials/MT_Electronic.MT_Electronic" "None"))
      (set `self.DMTI_sphere` _returnvalue))))