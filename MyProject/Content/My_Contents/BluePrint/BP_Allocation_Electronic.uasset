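; BP_Allocation_Electronic is a placement volume that scatters BP_P_Electronic actors, the game's electrons, at random points inside a box when play begins.
; The construction script adds a non-colliding box component to visualize the area, sized by BoxExtent and offset by that extent so the actor's origin sits at a corner.
; BeginPlay spawns GenNum electrons within that box's bounds at the configured Scale, regardless of collisions.
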(event `self.ReceiveBeginPlay`
  (bind (_origin _boxextent) (`KismetSystemLibrary.GetComponentBounds` (`self.Box_Collision`)))
  ;[1 1 1] 範囲内に電子を生成
  (for _ (range 1 (+ (`self.gen_num`) 1))
    (`|SpawnActorFromClass` "/Game/My_Contents/BluePrint/BP_P_Electronic.BP_P_Electronic_C" (`KismetMathLibrary.MakeTransform` (`KismetMathLibrary.RandomPointInBoundingBox` _origin _boxextent) (struct) (`self.Scale`)) "AlwaysSpawn" "OverrideRootScale" null null)))

(fn `UserConstructionScript`
  (bind _box_collision (`self.Box_Collision`))
  ;[1 1 1] Box_Collision(当たり判定無しの範囲を視覚化する為のBox)を生成
  (bind _returnvalue (`AddComponent|NODE_AddBoxComponent-0` :`bManualAttachment` true))
  (set `self.Box_Collision` _returnvalue)
  (`SceneComponent.K2_AttachToComponent` _box_collision (`self.DefaultSceneRoot`) "None" "KeepRelative" "KeepRelative" "KeepRelative" true)
  (`BoxComponent.SetBoxExtent` _box_collision (`self.Box_Extent`) true)
  (`SceneComponent.K2_AddRelativeLocation` _box_collision (`self.Box_Extent`) false false))