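; BP_Electronic_Exploation is an actor, apparently a short-lived explosion effect, that launches the arrows of overlapping BP_P_Electronic actors.
; On BeginPlay it attaches to a supplied parent component and socket, then checks its overlaps once.
; Each Arrow gets physics and a velocity-change impulse along its AttachingSpringarm's forward axis.
; The actor destroys itself inside the loop before a Delay, so the following physics shutoff likely never runs.
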(event `self.ReceiveBeginPlay`
  (`self.K2_AttachToComponent` (`self.parent_component`) (`self.soclet_name`) "SnapToTarget" "KeepWorld" "KeepWorld")
  (for _array_element (`self.GetOverlappingActors` "/Game/My_Contents/BluePrint/BP_P_Electronic.BP_P_Electronic_C")
    (bind _asbp_p_electronic (cast `/Game/My_Contents/BluePrint/BP_P_Electronic` _array_element))
    (bind _arrow (`/Game/My_Contents/BluePrint/BP_P_Electronic.Arrow` _asbp_p_electronic))
    (`PrimitiveComponent.SetSimulatePhysics` _arrow true)
    (`PrimitiveComponent.AddImpulse` _arrow (* (`KismetMathLibrary.Normal` (`KismetMathLibrary.Conv_RotatorToVector` (`SceneComponent.K2_GetComponentRotation` (`/Game/My_Contents/BluePrint/BP_P_Electronic.attaching_springarm` _asbp_p_electronic)))) 10.0) "None" true)
    (`self.K2_DestroyActor`)
    (`KismetSystemLibrary.Delay` 1.0)
    (`PrimitiveComponent.SetSimulatePhysics` _arrow false)))

(event `self.ReceiveTick`
  (params (DeltaSeconds :type "Float (single-precision)")))

(fn `UserConstructionScript`)

(fn `新規関数_0`)