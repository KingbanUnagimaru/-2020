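; Generator that spawns a BP_Shinnkai electron-attracting sphere on the player's socket when MakeShinnkai is set.
; Tick starts a timeline that expands the sphere, and on the player's jump destroys it and spawns BP_Electronic_Explosion.
; A looping timer clears finished lightning emitters and, once none remain, spawns a new batch reaching to the sphere's bounds.
; Batch size comes from ten percentage bands of the sphere's GenNum/GenNumLimit ratio.
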(event `self.ReceiveBeginPlay`
  (`|ExecutionSequence`
    (:`then_0`
      (bind _asbp_player (cast `/Game/Miya/Player/BP_Player` (`GameplayStatics.GetPlayerPawn` 0)))
      (set `self.Player` _asbp_player))))

(event `CE_Spawn_Random_Lightning`
  (bind _lightning_emmitter (`self.lightning_emmitter`))
  (`|ExecutionSequence`
    (:`then_0`
      (if (`KismetArrayLibrary.Array_IsValidIndex` (`self.lightning_emmitter`))
        (for (_array_element _array_index) _lightning_emmitter
          (if (not (`ActorComponent.IsActive` _array_element))
            (`ActorComponent.K2_DestroyComponent` _array_element)
            (`KismetArrayLibrary.Array_Remove` _lightning_emmitter _array_index)))))
    (:`then_1`
      (`self.Spawn_Random_Lightning` 1 2 3 4 5 6 7 8 9 15))))

(event `self.ReceiveTick`
  (params (DeltaSeconds :type "Float (single-precision)"))
  (bind _shinnkai (`self.Shinnkai`))
  (bind _player (`self.Player`))
  (bind _player_2 (`self.Player`))
  ;[1 1 1] 生成したShinnkaiを段々と膨張させる処理
  (`|ExecutionSequence`
    (:`then_0`
      (if (`KismetSystemLibrary.IsValid` _player_2)
        (if (`/Game/Miya/Player/BP_Player.MakeShinnkai` _player_2)
          (`|ExecutionSequence`
            (:`then_0`
              (if (not (`self.shinkai_gen_flag`))
                ;[1 1 1] 電子を引き寄せるトリガーとなる球（Shinnkai）を生成してターゲットにアタッチ
                (bind _returnvalue (`|SpawnActorFromClass` "/Game/My_Contents/BluePrint/BP_Shinnkai.BP_Shinnkai_C" (`self.Shinnkai_initial_T`) "AlwaysSpawn" "OverrideRootScale" null null))
                (set `self.Shinnkai` _returnvalue)
                (`SceneComponent.SetWorldScale3D` (`/Game/My_Contents/BluePrint/BP_Shinnkai.Sphere` _shinnkai) (`self.Shinkai_scale`))
                (`self.K2_AttachToComponent` _shinnkai (`/Game/Miya/Player/BP_Player.Sphere` (cast `/Game/Miya/Player/BP_Player` (`self.Target_Mesh`) :!pure true)) (`self.Socket_name`) "SnapToTarget" "KeepWorld" "KeepWorld" true)
                (set `self.shinkai_gen_flag` true)
                (set `/Game/My_Contents/BluePrint/BP_Shinnkai.Gen_shinnkai` self (`self.Shinnkai`))
                (bind _returnvalue_2 (`KismetSystemLibrary.K2_SetTimerDelegate` (delegate `CE_Spawn_Random_Lightning`) 0.01 true))
                (set `self.th_spawn_random_lightning` _returnvalue_2)
                (set `/Game/Miya/Player/BP_Player.MakeShinnkai` false (`self.Player`))
                ;[1 1 1] Shinnkaiを削除する処理
                (if (`/Game/Miya/Player/BP_Player.DidJump` _player) :!label _label
                  (set `self.shinkai_gen_flag` false)
                  (`self.OnDestroyShinnkai`)
                  (`self.K2_DestroyActor` (`self.Shinnkai`))
                  (`|SpawnActorFromClass` "/Game/My_Contents/BluePrint/BP_Electronic_Explosion.BP_Electronic_Explosion_C" (`KismetMathLibrary.MakeTransform` (0.0 0.0 0.0) (struct) (* (1.0 1.0 1.0) (`self.explosion_scale`))) "AlwaysSpawn" "OverrideRootScale" null (`/Game/Miya/Player/BP_Player.Sphere` (cast `/Game/Miya/Player/BP_Player` (`self.Target_Mesh`) :!pure true)) (`self.Socket_name`) null)
                  (`KismetSystemLibrary.K2_ClearAndInvalidateTimerHandle` (`self.th_spawn_random_lightning`))
                  (set `/Game/Miya/Player/BP_Player.DidJump` false _player))
                (if (`self.shinkai_gen_flag`)
                  (`/Engine/EditorBlueprintResources/StandardMacros.DoOnce` false :!label _label_2
                    (:`Completed`
                      (bind (_direction _expansion_speed) (`Timeline|TL_Expansion_Speed` :!via `PlayFromStart` :!label _label_3)
                        (:`Update`
                          (set `self.Shinkai_scale` (`KismetMathLibrary.MakeVector` _expansion_speed _expansion_speed _expansion_speed))
                          (`SceneComponent.SetWorldScale3D` (`/Game/My_Contents/BluePrint/BP_Shinnkai.Sphere` (`self.Shinnkai`)) (`self.Shinkai_scale`))))))
                  (else
                    (`|ExecutionSequence`
                      (:`then_0`
                        (goto _label_2 :!via `Reset`))
                      (:`then_1`
                        (goto _label_3 :!via `Stop`))))))))
          (else
            (goto _label)))))))

(fn `Spawn_Random_Lightning`
  (params (`0<x<=10` :type Integer) (`10<x<=20` :type Integer) (`20<x<=30` :type Integer) (`30<x<=40` :type Integer) (`40<x<=50` :type Integer) (`50<x<=60` :type Integer) (`60<x<=70` :type Integer) (`70<x<=80` :type Integer) (`80<x<=90` :type Integer) (`90<x<=100` :type Integer))
  (locals (`L_0<x<=10` :type Integer) (`L_10<x<=20` :type Integer) (`L_20<x<=30` :type Integer) (`L_30<x<=40` :type Integer) (`L_40<x<=50` :type Integer) (`L_50<x<=60` :type Integer) (`L_60<x<=70` :type Integer) (`L_70<x<=80` :type Integer) (`L_80<x<=90` :type Integer) (`L_90<x<=100` :type Integer) (L_gen_num :type Integer))
  (bind _shinnkai (`self.Shinnkai`))
  (bind _shinnkai_2 (`self.Shinnkai`))
  (bind _returnvalue (* (/ (`KismetMathLibrary.Conv_IntToDouble` (`/Game/My_Contents/BluePrint/BP_Shinnkai.Gen_num` _shinnkai_2)) (`KismetMathLibrary.Conv_IntToDouble` (`/Game/My_Contents/BluePrint/BP_Shinnkai.Gen_num_limit` _shinnkai_2))) 100.0))
  (`|ExecutionSequence`
    (:`then_0`
      (set `local.L_0<x<=10` `0<x<=10`))
    (:`then_1`
      (set `local.L_10<x<=20` `10<x<=20`))
    (:`then_2`
      (set `local.L_20<x<=30` `20<x<=30`))
    (:`then_3`
      (set `local.L_30<x<=40` `30<x<=40`))
    (:`then_4`
      (set `local.L_40<x<=50` `40<x<=50`))
    (:`then_5`
      (set `local.L_50<x<=60` `50<x<=60`))
    (:`then_6`
      (set `local.L_60<x<=70` `60<x<=70`))
    (:`then_7`
      (set `local.L_70<x<=80` `70<x<=80`))
    (:`then_8`
      (set `local.L_80<x<=90` `80<x<=90`))
    (:`then_9`
      (set `local.L_90<x<=100` `90<x<=100`))
    (:`then_10`
      (if (`KismetSystemLibrary.IsValid` _shinnkai_2)
        (`|ExecutionSequence`
          (:`then_0`
            (if (and (> _returnvalue 0.0) (<= _returnvalue 10.0))
              (set `local.L_gen_num` (`local.L_0<x<=10`))))
          (:`then_1`
            (if (and (> _returnvalue 10.0) (<= _returnvalue 20.0))
              (set `local.L_gen_num` (`local.L_10<x<=20`))))
          (:`then_2`
            (if (and (> _returnvalue 20.0) (<= _returnvalue 30.0))
              (set `local.L_gen_num` (`local.L_20<x<=30`))))
          (:`then_3`
            (if (and (> _returnvalue 30.0) (<= _returnvalue 40.0))
              (set `local.L_gen_num` (`local.L_30<x<=40`))))
          (:`then_4`
            (if (and (> _returnvalue 40.0) (<= _returnvalue 50.0))
              (set `local.L_gen_num` (`local.L_40<x<=50`))))
          (:`then_5`
            (if (and (> _returnvalue 50.0) (<= _returnvalue 60.0))
              (set `local.L_gen_num` (`local.L_50<x<=60`))))
          (:`then_6`
            (if (and (> _returnvalue 60.0) (<= _returnvalue 70.0))
              (set `local.L_gen_num` (`local.L_60<x<=70`))))
          (:`then_7`
            (if (and (> _returnvalue 70.0) (<= _returnvalue 80.0))
              (set `local.L_gen_num` (`local.L_70<x<=80`))))
          (:`then_8`
            (if (and (> _returnvalue 80.0) (<= _returnvalue 90.0))
              (set `local.L_gen_num` (`local.L_80<x<=90`))))
          (:`then_9`
            (if (and (> _returnvalue 90.0) (<= _returnvalue 100.0))
              (set `local.L_gen_num` (`local.L_90<x<=100`))))
          (:`then_10`
            (if (not (`KismetArrayLibrary.Array_IsValidIndex` (`self.lightning_emmitter`)))
              (for _ (range 1 (+ (`local.L_gen_num`) 1))
                (bind _returnvalue_2 (`GameplayStatics.SpawnEmitterAttached` "/Game/My_Contents/Particle/P_Lighting.P_Lighting" (`/Game/Miya/Player/BP_Player.Sphere` (cast `/Game/Miya/Player/BP_Player` (`self.Target_Mesh`) :!pure true)) (`self.Socket_name`) (0.0 0.0 0.0) (`KismetMathLibrary.RandomRotator` false) (1.0 1.0 1.0) "SnapToTarget" false))
                (`KismetArrayLibrary.Array_Add` (`self.lightning_emmitter`) _returnvalue_2)
                (if (`KismetSystemLibrary.IsValid` _shinnkai)
                  (`FXSystemComponent.SetVectorParameter` _returnvalue_2 "target_point" (`KismetMathLibrary.MakeVector` (.x (`.BoxExtent` (`KismetSystemLibrary.GetComponentBounds` (`/Game/My_Contents/BluePrint/BP_Shinnkai.Sphere` _shinnkai)))))))))))))))

(fn `UserConstructionScript`)