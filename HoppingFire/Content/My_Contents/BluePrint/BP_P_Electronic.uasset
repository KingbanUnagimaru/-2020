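; Electron pawn driven by an AI behavior tree, with blackboard flags tracking attachment and explosion state.
; BeginPlay initializes BB_Electronic and runs the tree, while Refresh resets attachment, target and overlap keys.
; The construction script snaps an overlap-only sphere to the arrow and gives it a dynamic material.
; Helpers supply overlapping actors and random points inside the owning BP_Allocation_Electronic's box; GetDestination is a zero-vector stub.
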(event `self.ReceiveBeginPlay`
  (bind _returnvalue (`AIBlueprintHelperLibrary.GetAIController` self))
  (bind _blackboardcomponent (`AIController.UseBlackboard` _returnvalue "/Game/My_Contents/BehaviorTree/BB_Electronic.BB_Electronic"))
  (`BlackboardComponent.SetValueAsBool` _blackboardcomponent (`self.n_is_attached`) false)
  (`BlackboardComponent.SetValueAsBool` _blackboardcomponent (`self.n_is_explosion`) false)
  (`AIController.RunBehaviorTree` _returnvalue (`self.My_BT`)))

(event `self.ReceiveTick`
  (params (DeltaSeconds :type "Float (single-precision)")))

(event `Refresh`
  (bind _returnvalue (`AIBlueprintHelperLibrary.GetBlackboard` self))
  (`BlackboardComponent.SetValueAsBool` _returnvalue (`self.n_is_attached`) false)
  (`BlackboardComponent.ClearValue` _returnvalue (`self.n_TargetObjectKey`))
  (`BlackboardComponent.ClearValue` _returnvalue (`self.n_is_overlapping`)))

(fn `Get_Destination`
  (returns (Destination :type "Vector Structure"))
  (return (0.0 0.0 0.0)))

(fn `Get_Overlapping_Actors`
  (returns (overlapping_actor :type "Array of Actor Object Reference"))
  (return (`self.GetOverlappingActors` self null)))

(fn `Get_Random_Location`
  (returns (random_location :type "Vector Structure"))
  (bind _asbp_allocation_electronic (cast `/Game/My_Contents/BluePrint/BP_Allocation_Electronic` (`self.GetOwner`)))
  (bind _box_collision (`/Game/My_Contents/BluePrint/BP_Allocation_Electronic.Get_Box_Collison` _asbp_allocation_electronic))
  (bind (_origin _boxextent) (`KismetSystemLibrary.GetComponentBounds` _box_collision))
  (return (`KismetMathLibrary.RandomPointInBoundingBox` _origin _boxextent)))

(fn `UserConstructionScript`
  (locals (NewLocalVar_0 :type "SphereComponent Object Reference"))
  (bind _sphere (`self.Sphere`))
  (`|ExecutionSequence`
    (:`then_0`
      ;[1 1 1] 電子の各種設定
      (`SceneComponent.K2_AttachToComponent` _sphere (`self.Arrow`) "None" "SnapToTarget" "SnapToTarget" "SnapToTarget" true)
      (`PrimitiveComponent.SetMaterial` _sphere 0 "/Game/My_Contents/Materials/MT_Opaque_Inst.MT_Opaque_Inst")
      (`PrimitiveComponent.SetCollisionResponseToAllChannels` _sphere "ECR_Overlap")
      (bind _returnvalue (`PrimitiveComponent.CreateDynamicMaterialInstance` _sphere 0 "/Game/My_Contents/Materials/MT_Electronic.MT_Electronic" "None"))
      (set `self.DMTI_sphere` _returnvalue))))