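; BP_Gen_Shinnkai generates and removes the Shinnkai, a sphere that triggers attraction of electrons.
; The Shinnkai input alternates via FlipFlop between spawning BP_Shinnkai attached to the player's Sphere and destroying it after calling OnDestroyShinnkai.
; While the sphere's flag is set, Tick starts a timeline once to gradually expand its world scale.
; Clearing the flag stops the timeline and resets the DoOnce.
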(event `InputAction|Shinnkai`
  (params (Key :type "Key Structure"))
  (bind _shinnkai (`self.Shinnkai`))
  (:`Pressed`
    (`/Engine/EditorBlueprintResources/StandardMacros.FlipFlop`
      (:`A`
        (`|ExecutionSequence`
          (:`then_0`
            (if (not (`self.shinkai_gen_flag`))
              ;[1 1 1] 電子を引き寄せるトリガーとなる球（Shinnkai）を生成してターゲットにアタッチ
              (bind _returnvalue (`|SpawnActorFromClass` "/Game/My_Contents/BluePrint/BP_Shinnkai.BP_Shinnkai_C" (`self.Shinnkai_initial_T`) "AlwaysSpawn" "OverrideRootScale" null null))
              (set `self.Shinnkai` _returnvalue)
              (`SceneComponent.SetWorldScale3D` (`/Game/My_Contents/BluePrint/BP_Shinnkai.Sphere` _shinnkai) (`self.Shinkai_scale`))
              (`self.K2_AttachToComponent` _shinnkai (`/Game/Miya/Player/BP_Player.Sphere` (cast `/Game/Miya/Player/BP_Player` (`self.Target_Mesh`) :!pure true)) (`self.Socket_name`) "SnapToTarget" "KeepWorld" "KeepWorld" true)
              (set `self.shinkai_gen_flag` true)
              (set `/Game/My_Contents/BluePrint/BP_Shinnkai.Gen_shinnkai` self (`self.Shinnkai`))))))
      (:`B`
        ;[1 1 1] Shinnkaiを削除する処理
        (set `self.shinkai_gen_flag` false)
        (`self.OnDestroyShinnkai`)
        (`self.K2_DestroyActor` (`self.Shinnkai`))))))

(event `self.ReceiveTick`
  (params (DeltaSeconds :type "Float (single-precision)"))
  ;[1 1 1] 生成したShinnkaiを段々と膨張させる処理
  (if (`self.shinkai_gen_flag`)
    (`/Engine/EditorBlueprintResources/StandardMacros.DoOnce` false :!label _label
      (:`Completed`
        (bind (_direction _expansion_speed) (`Timeline|TL_Expansion_Speed` :!via `PlayFromStart` :!label _label_2)
          (:`Update`
            (set `self.Shinkai_scale` (`KismetMathLibrary.MakeVector` _expansion_speed _expansion_speed _expansion_speed))
            (`SceneComponent.SetWorldScale3D` (`/Game/My_Contents/BluePrint/BP_Shinnkai.Sphere` (`self.Shinnkai`)) (`self.Shinkai_scale`))))))
    (else
      (`|ExecutionSequence`
        (:`then_0`
          (goto _label :!via `Reset`))
        (:`then_1`
          (goto _label_2 :!via `Stop`))))))

(fn `UserConstructionScript`)