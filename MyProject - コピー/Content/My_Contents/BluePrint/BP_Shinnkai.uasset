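; BP_Shinnkai is an actor that captures overlapping BP_P_Electronic actors up to a count limit.
; Each Tick below the limit, it flags their blackboards and passes itself as the object value.
; AttachSpringarm claims an unattached target, creating a collision-free spring arm with negative length aimed at it, attaching it and storing the arm on it.
; At the limit, AttachSpringarm clears the target's flag and object keys instead.
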(event `self.ReceiveTick`
  (params (DeltaSeconds :type "Float (single-precision)"))
  (if (< (`self.Gen_num`) (`self.Gen_num_limit`))
    (for _array_element (`self.GetOverlappingActors` self "/Game/My_Contents/BluePrint/BP_P_Electronic.BP_P_Electronic_C")
      (bind _returnvalue (`AIBlueprintHelperLibrary.GetBlackboard` _array_element))
      (`BlackboardComponent.SetValueAsBool` _returnvalue (`self.NewVar_1`) true)
      (`BlackboardComponent.SetValueAsObject` _returnvalue (`self.NewVar_2`) self))))

(event `/Game/My_Contents/BluePrint/BP_Masayuki_Interface.Attach_Springarm`
  (params (Attach_target :type "Actor Object Reference"))
  (bind _returnvalue (`self.K2_GetActorLocation`))
  (bind _returnvalue_2 (`self.K2_GetActorLocation` Attach_target))
  (bind _returnvalue_3 (`AIBlueprintHelperLibrary.GetBlackboard` Attach_target))
  (bind _gen_num (`self.Gen_num`))
  (bind _newvar_3 (`self.NewVar_3`))
  (if (`BlackboardComponent.GetValueAsBool` _returnvalue_3 _newvar_3)
    _
    (elif (< _gen_num (`self.Gen_num_limit`))
      (set `self.Gen_num` (+ _gen_num 1))
      (`BlackboardComponent.SetValueAsBool` _returnvalue_3 _newvar_3 true)
      (bind _returnvalue_4 (`AddComponent|NODE_AddSpringArmComponent-0` :`bManualAttachment` true :`RelativeTransform` (`KismetMathLibrary.MakeTransform` (0.0 0.0 0.0) (`KismetMathLibrary.FindLookAtRotation` _returnvalue _returnvalue_2))))
      (set `SpringArmComponent.bDoCollisionTest` false _returnvalue_4)
      (set `SpringArmComponent.bInheritPitch` false _returnvalue_4)
      (set `SpringArmComponent.bInheritRoll` false _returnvalue_4)
      (set `SpringArmComponent.bInheritYaw` false _returnvalue_4)
      (set `SpringArmComponent.TargetArmLength` (* (`KismetMathLibrary.Abs` (`KismetMathLibrary.VSize` (- _returnvalue_2 _returnvalue))) -1.0) _returnvalue_4)
      (`SceneComponent.K2_AttachToComponent` _returnvalue_4 (`self.DefaultSceneRoot`) "None" "SnapToTarget" "KeepRelative" "KeepRelative" false)
      (`self.K2_AttachToComponent` Attach_target _returnvalue_4 "None" "SnapToTarget" "KeepWorld" "KeepWorld" false)
      (bind _asbp_p_electronic (cast `/Game/My_Contents/BluePrint/BP_P_Electronic` Attach_target))
      (set `/Game/My_Contents/BluePrint/BP_P_Electronic.attaching_springarm` _returnvalue_4 _asbp_p_electronic)
      (else
        (`BlackboardComponent.ClearValue` _returnvalue_3 (`self.NewVar_1`))
        (`BlackboardComponent.ClearValue` _returnvalue_3 (`self.NewVar_2`))))))

(fn `Get_Destination`
  (returns (Destination :type "Vector Structure"))
  (return (0.0 0.0 0.0)))

(fn `Get_Overlapping_Actors`
  (returns (overlapping_actor :type "Array of Actor Object Reference"))
  (return))

(fn `Get_Random_Location`
  (returns (random_location :type "Vector Structure"))
  (return (0.0 0.0 0.0)))

(fn `UserConstructionScript`)