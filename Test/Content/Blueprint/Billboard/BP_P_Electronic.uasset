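; BP_P_Electronic is a glowing, colored billboard actor with sphere collision, built entirely in the construction script.
; It adds an instanced plane with a dynamic billboard material tinted by Color, leaving the billboarding to that material.
; A collision sphere sized from the plane mesh bounds and a point light matching the material color are snapped to the same Arrow as the plane.
; The event graph holds no logic.
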(event `self.ReceiveTick`
  (params (DeltaSeconds :type "Float (single-precision)")))

(fn `UserConstructionScript`
  (bind _ism_plane (`self.ISM_Plane`))
  (bind _ism_plane_2 (`self.ISM_Plane`))
  (`|ExecutionSequence`
    (:`then_0`
      ;[1 1 1] 板のインスタンス生成しビルボード処理を施す
      (bind _returnvalue (`AddComponent|NODE_AddInstancedStaticMeshComponent-0` :`bManualAttachment` true :`RelativeTransform` (`self.ISM_Plane_Relative_Transform`)))
      (set `self.ISM_Plane` _returnvalue)
      (`SceneComponent.K2_AttachToComponent` _returnvalue (`self.Arrow`) "None" "SnapToTarget" "SnapToTarget" "SnapToTarget" true)
      (`StaticMeshComponent.SetStaticMesh` _ism_plane_2 (`self.Plane`))
      (bind _returnvalue_2 (`PrimitiveComponent.CreateDynamicMaterialInstance` _ism_plane_2 0 (`self.MT_Billboard`) "None"))
      (set `self.DMT_Billboard` _returnvalue_2)
      (`InstancedStaticMeshComponent.AddInstance` _ism_plane (`self.ISM_Plane_Relative_Transform`))
      (`PrimitiveComponent.SetCastShadow` _ism_plane false)
      (`MaterialInstanceDynamic.SetVectorParameterValue` (`self.DMT_Billboard`) "BaseColor" (`self.Color`)))
    (:`then_1`
      ;[1 1 1] 球の当たり判定を生成
      (bind _returnvalue_3 (`AddComponent|NODE_AddSphereComponent-0` :`bManualAttachment` true))
      (bind _output_get (set `self.Sphere_Collison` _returnvalue_3))
      (`SphereComponent.SetSphereRadius` _output_get (.y (`.BoxExtent` (`KismetMathLibrary.BreakBoxSphereBounds` (`StaticMesh.GetBounds` (`self.Plane`))))) true)
      (`SceneComponent.K2_AttachToComponent` _output_get (`self.Arrow`) "None" "SnapToTarget" "SnapToTarget" "SnapToTarget" true)
      (`PrimitiveComponent.SetCastShadow` (`self.Sphere_Collison`) false))
    (:`then_2`
      ;[1 1 1] 発光処理
      (bind _returnvalue_4 (`AddComponent|NODE_AddPointLightComponent-0` :`bManualAttachment` true))
      (bind _output_get_2 (set `self.Emmison` _returnvalue_4))
      (`LightComponent.SetIntensity` _output_get_2 (`self.Intensity`))
      (`LocalLightComponent.SetAttenuationRadius` _output_get_2 (`self.Attennuation_Radius`))
      (bind _returnvalue_5 (`MaterialInstanceDynamic.K2_GetVectorParameterValue` (`self.DMT_Billboard`) "BaseColor"))
      (`LightComponent.SetLightColor` _output_get_2 _returnvalue_5 true)
      (`PointLightComponent.SetSourceRadius` _output_get_2 0.0)
      (`SceneComponent.K2_AttachToComponent` _output_get_2 (`self.Arrow`) "None" "SnapToTarget" "SnapToTarget" "SnapToTarget" true))))